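; Trigger actor that changes the camera framing of the arcade player car when it drives through.
; On overlap by an actor with a Player-tagged component, it casts to carRayBP_duplicate and eases the car's SpringArm rotation by RotationToApply over one second.
; A Return flag alternates between two timelines that animate the arm length out and back on successive passes.
; The rotation offset is added on every pass, not reversed.
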(event Collision|EventActorBeginOverlap
  (params (OtherActor :type Actor%20Object%20Reference))
  (if (Utilities|Array|IsValidIndex (Actor|GetComponentsbyTag OtherActor "/Script/Engine.ActorComponent" "Player"))
    (bind _ascar_ray_bp_duplicate (Utilities|Casting|CastTocarRayBP_duplicate OtherActor))
    (Components|MoveComponentTo (Variables|/Game/VehicleArcade/carRayBP_duplicate.carRayBP_duplicate_C|GetSpringArm _ascar_ray_bp_duplicate) "0, 0, 0" (Math|Rotator|CombineRotators (Variables|/Script/Engine.SceneComponent|GetRelativeRotation (Variables|/Game/VehicleArcade/carRayBP_duplicate.carRayBP_duplicate_C|GetSpringArm _ascar_ray_bp_duplicate)) (Variables|Default|GetrotationToApply)) true false 1.0 false)
    (if (Variables|Default|Getreturn)
      (bind _returnspringarmtrack (Timeline|Timeline_0 PlayFromStart)
        (:Update
          (Variables|/Script/Engine.SpringArmComponent|SetTargetArmLength (Variables|/Game/VehicleArcade/carRayBP_duplicate.carRayBP_duplicate_C|GetSpringArm _ascar_ray_bp_duplicate) _returnspringarmtrack))
        (:Finished
          (Variables|Default|Setreturn false)))
      (else
        (bind _springarmtrack (Timeline|SpringArmDistance PlayFromStart)
          (:Update
            (Variables|/Script/Engine.SpringArmComponent|SetTargetArmLength (Variables|/Game/VehicleArcade/carRayBP_duplicate.carRayBP_duplicate_C|GetSpringArm _ascar_ray_bp_duplicate) _springarmtrack))
          (:Finished
            (Variables|Default|Setreturn true)))))))

(event EventBeginPlay
  (Variables|Default|Setreturn false))

(fn ConstructionScript)