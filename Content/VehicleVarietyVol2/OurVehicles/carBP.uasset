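; Car Blueprint that drives a physics Box forward and back from the MoveForward input axis.
; Each Tick applies a velocity-change impulse to the Box along the Cube's forward vector, scaled by MoveSpeed and delta time.
; Steering is unfinished: a Direction vector is computed from MoveRight, SteeringAngle and the Box's up vector but never applied, and the rotation nodes are left unconnected.
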(event EventTick
  (params (DeltaSeconds :type Float%20%28single-precision%29))
  (Utilities|FlowControl|Sequence
    (:then_0
      (bind _output_get (Variables|Default|SetmoveForward (* (Input|AxisValues|GetMoveForward) (Variables|Default|GetmoveSpeed) (Math|Vector|GetForwardVector (Variables|Default|GetCube)) DeltaSeconds)))
      (Physics|AddImpulse (Variables|Default|GetBox) _output_get "None" true))
    (:then_1
      (Variables|Default|Setdirection (* (Math|Vector|GetUpVector (Variables|Default|GetBox)) (Input|AxisValues|GetMoveRight) (Variables|Default|GetsteeringAngle) DeltaSeconds)))))

(fn ConstructionScript)