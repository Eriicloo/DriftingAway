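; BP_SUV_Chaos is a player-drivable SUV vehicle pawn, apparently using Chaos vehicle physics.
; Input axes feed throttle, brake and steering into the vehicle movement component, while Turn and LookUp rotate the controller view.
; The handbrake also triggers a one-shot yaw spin on the mesh from Tick, setting angular velocity from steering (stored as "Thortle") scaled by the actor's yaw captured at press.
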(event EventTick
  (params (DeltaSeconds :type Float%20%28single-precision%29))
  (if (Variables|Default|GetIs%20Handbrake%20on?)
    (if (not (Variables|Default|GetaplyRotation))
      (Variables|Default|SetaplyRotation true)
      (Class|PrimitiveComponent|SetPhysicsAngularVelocityinDegrees (Variables|Character|GetMesh) (Math|Vector|MakeVector 0.0 0.0 (* (* (Variables|Default|Getthortle) 1e+01) (.yaw (Variables|Default|GetRotateActor)))) false "None"))
    (else
      (Variables|Default|SetaplyRotation false))))

(event Input|ActionEvents|InputActionHandbrake
  (params (Key :type Key%20Structure :default "None"))
  (bind _vehiclemovementcomponent (Variables|Default|GetVehicleMovementComponent))
  (:Pressed
    (Variables|Default|SetRotateActor (Transformation|GetActorRotation))
    (Class|ChaosVehicleMovementComponent|SetHandbrakeInput _vehiclemovementcomponent true)
    (Variables|Default|SetIs%20Handbrake%20on? true))
  (:Released
    (Class|ChaosVehicleMovementComponent|SetHandbrakeInput _vehiclemovementcomponent false)
    (Variables|Default|SetIs%20Handbrake%20on? false)))

(event Input|AxisEvents|InputAxisMoveRight
  (params (AxisValue :type Float%20%28single-precision%29))
  (bind _output_get (Variables|Default|Setthortle AxisValue))
  (Class|ChaosVehicleMovementComponent|SetSteeringInput (Variables|Default|GetVehicleMovementComponent) _output_get))

(event Input|AxisEvents|InputAxisTurn
  (params (AxisValue :type Float%20%28single-precision%29))
  (Pawn|Input|AddControllerYawInput AxisValue))

(event Input|AxisEvents|InputAxisLookUp
  (params (AxisValue :type Float%20%28single-precision%29))
  (Pawn|Input|AddControllerPitchInput AxisValue))

(event Input|AxisEvents|InputAxisMoveForward
  (params (AxisValue :type Float%20%28single-precision%29))
  (Class|ChaosVehicleMovementComponent|SetThrottleInput (Variables|Default|GetVehicleMovementComponent) AxisValue))

(event Input|AxisEvents|InputAxisReverse/Brake
  (params (AxisValue :type Float%20%28single-precision%29))
  (Class|ChaosVehicleMovementComponent|SetBrakeInput (Variables|Default|GetVehicleMovementComponent) AxisValue))

(fn ConstructionScript)